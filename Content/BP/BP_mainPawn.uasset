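; Player pawn that acts as the keyboard input layer for a game where figures are moved and rotated, apparently a falling-block puzzle.
; Arrow key events cast the game mode to MyGameMode and call it to move the figure left or right or rotate it.
; Holding Down forces faster descent, and releasing it restores normal movement.
; The pawn holds no game logic itself, leaving all figure handling to the game mode.
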(event `Key|Left`
  (params (Key :type "Key Structure"))
  (:`Pressed`
    (bind _asmy_game_mode (cast `/Game/MyGameMode` (`GameplayStatics.GetGameMode`)))
    (`/Game/MyGameMode.MoveFigureLeft` _asmy_game_mode "NewEnumerator0")))

(event `Key|Right`
  (params (Key :type "Key Structure"))
  (:`Pressed`
    (bind _asmy_game_mode (cast `/Game/MyGameMode` (`GameplayStatics.GetGameMode`)))
    (`/Game/MyGameMode.MoveFigureRight` _asmy_game_mode "NewEnumerator1")))

(event `Key|Up`
  (params (Key :type "Key Structure"))
  (:`Pressed`
    (bind _asmy_game_mode (cast `/Game/MyGameMode` (`GameplayStatics.GetGameMode`)))
    (`/Game/MyGameMode.RotateFigure` _asmy_game_mode)))

(event `Key|Down`
  (params (Key :type "Key Structure"))
  (bind _returnvalue (`GameplayStatics.GetGameMode`))
  (:`Pressed`
    (bind _asmy_game_mode (cast `/Game/MyGameMode` _returnvalue))
    (`/Game/MyGameMode.MoveDownForce` _asmy_game_mode))
  (:`Released`
    (bind _asmy_game_mode_2 (cast `/Game/MyGameMode` _returnvalue))
    (`/Game/MyGameMode.MoveDownNormal` _asmy_game_mode_2)))

(fn `UserConstructionScript`)