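; BP_cube is a grid-positioned cube actor with floating and dead material states.
; SetPosition stores a 2D coordinate and maps it to world Y and Z in 100-unit cells.
; BeginPlay places the cube, then tints a dynamic instance of the floating material with two colors loaded from the SettingsSave slot.
; Helper functions switch to the dead or untinted floating material, though the event graph's SetFloatingMaterial call is disconnected.
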(event `self.ReceiveBeginPlay`
  (`self.SetPosition` (`self.Position`))
  (bind _returnvalue (`GameplayStatics.LoadGameFromSlot` "SettingsSave"))
  (bind _assettings_save (cast `/Game/Settings/SettingsSave` _returnvalue))
  (bind _returnvalue_2 (`KismetMaterialLibrary.CreateDynamicMaterialInstance` (`self.FloatingMaterial`)))
  (`MaterialInstanceDynamic.SetVectorParameterValue` _returnvalue_2 "ColorA" (`/Game/Settings/SettingsSave.ColorA` _assettings_save))
  (`MaterialInstanceDynamic.SetVectorParameterValue` _returnvalue_2 "ColorB" (`/Game/Settings/SettingsSave.ColorB` _assettings_save))
  (`PrimitiveComponent.SetMaterial` (`self.Cube`) 0 _returnvalue_2))

(event `self.ReceiveTick`
  (params (DeltaSeconds :type "Float (single-precision)")))

(fn `SetDeadMaterial`
  (`PrimitiveComponent.SetMaterial` (`self.Cube`) 0 (`self.DeadMaterial`)))

(fn `SetFloatingMaterial`
  (`PrimitiveComponent.SetMaterial` (`self.Cube`) 0 (`self.FloatingMaterial`)))

(fn `SetPosition`
  (params (Pos :type "IntPoint Structure"))
  (bind _output_get (set `self.Position` Pos))
  (bind (_x _y) (break `IntPoint` _output_get))
  (`self.K2_SetActorLocation` (`KismetMathLibrary.MakeVector` 0.0 (`KismetMathLibrary.Conv_IntToDouble` (* _x 100)) (`KismetMathLibrary.Conv_IntToDouble` (* _y 100)))))

(fn `UserConstructionScript`)